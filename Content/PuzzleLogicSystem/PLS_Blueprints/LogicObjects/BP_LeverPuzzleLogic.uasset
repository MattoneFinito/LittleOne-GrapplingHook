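; Puzzle logic lever that toggles on an Activate state, swinging its handle by timeline and sending Activate or Deactivate to linked actors when the swing finishes.
; Optional auto-deactivation counts down in Tick on two coloured text renders, then re-enters the toggle logic to swing back.
; Interaction is blocked during movement or countdown, with cooldown and timeline play rate derived from the rotation duration.
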(event `self.ReceiveBeginPlay`
  ;[1 1 1] Set timeline playrate. Set cooldown to slightly longer than the lever rotation duration.
  (`parent.ReceiveBeginPlay`)
  (`TimelineComponent.SetPlayRate` (`self.TimelineRotateLever`) (/ 1.0 (`self.RotateDuration`)))
  (set `self.InteractionCooldown` (+ (`self.RotateDuration`) 0.05)))

(event `/Game/PuzzleLogicSystem/PLS_Blueprints/Misc/BPI_PuzzleLogic.OnEnterState`
  (params (State :type "/Game/PuzzleLogicSystem/PLS_Blueprints/Misc/ENUM_LogicTriggerStates Enum" :default "NewEnumerator0"))
  ;[1 1 1] Puzzle logic event received to activate the lever.
  ; Triggers linked actors when the lever completes its rotating animation.
  (`parent.OnEnterState` State)
  (switch `/Game/PuzzleLogicSystem/PLS_Blueprints/Misc/ENUM_LogicTriggerStates` State
    (:`NewEnumerator0`
      (if (not (`self.IsCurrentlyActive`))
        (if (`self.InActiveState`)
          (set `self.LeverRotateMultiplier` 2.0 :!label _label)
          (set `self.InActiveState` false)
          (else
            (set `self.LeverRotateMultiplier` -2.0)
            (set `self.InActiveState` true)))
        (set `self.Moving` true)
        (`GameplayStatics.PlaySoundAtLocation` (`self.ActivateSFX`) (`self.K2_GetActorLocation`) (struct) 1.0 1.0 0.0 null null null null)
        (`Timeline|TimelineRotateLever` :!via `PlayFromStart`
          (:`Update`
            (`SceneComponent.K2_AddLocalRotation` (`self.LeverHandle`) (`KismetMathLibrary.MakeRotator` 0.0 (* (`GameplayStatics.GetWorldDeltaSeconds`) (* (`self.LeverSpeed`) (`self.LeverRotateMultiplier`)))) false false))
          (:`Finished`
            (set `self.Moving` false)
            (if (`self.InActiveState`)
              (`self.TriggerLinkedActors` "NewEnumerator0")
              (if (`self.AutoDeactivate`)
                (set `self.DeactivateTimer_Internal` (`self.AutoDeactivateTimer`))
                (`TextRenderComponent.SetTextRenderColor` (`self.TextRender`) (`self.ActiveColour`))
                (`TextRenderComponent.SetTextRenderColor` (`self.TextRender2`) (`self.ActiveColour`)))
              (else
                (`self.TriggerLinkedActors` "NewEnumerator1")
                (`self.SetTimerText` (`self.AutoDeactivateTimer`))
                (`TextRenderComponent.SetTextRenderColor` (`self.TextRender`) (`self.InactiveColour`))
                (`TextRenderComponent.SetTextRenderColor` (`self.TextRender2`) (`self.InactiveColour`))))))))
    (:`NewEnumerator16`
      (`PrimitiveComponent.SetCollisionEnabled` (`self.InteractCollision`) "NoCollision"))))

(event `self.ReceiveTick`
  (params (DeltaSeconds :type "Float (single-precision)"))
  ;[1 1 1] Logic for handling auto-deactivation.
  ; Auto-deactivation means that the lever automatically deactivates after a certain amount of time.
  (`parent.ReceiveTick` DeltaSeconds)
  (if (> (`self.DeactivateTimer_Internal`) 0.0)
    (bind _output_get (set `self.DeactivateTimer_Internal` (- (`self.DeactivateTimer_Internal`) DeltaSeconds)))
    (if (<= _output_get 0.0)
      (goto _label)
      (else
        (`self.SetTimerText` (`self.DeactivateTimer_Internal`))))))

(fn `IsCurrentlyActive`
  (returns (IsAuto :type Boolean))
  ;[1 1 1] Returns whether the lever is currently animating, or whether it has been activated
  ; and is currently counting down to auto-deactivate.
  (return (or (> (`self.DeactivateTimer_Internal`) 0.0) (`self.Moving`))))

(fn `IsValidInteractObject`
  (returns (IsValid :type Boolean))
  ;[1 1 1] In addition to basic checks for valid interaction, also makes sure the lever is not currently animating.
  ; Ie. The lever cannot be interacted with while it is already rotating.
  (return (and (`parent.IsValidInteractObject`) (not (`self.IsCurrentlyActive`)))))

(fn `SetTimerText`
  (params (Time :type "Float (double-precision)"))
  ;[1 1 1] Update the auto-deactivate timer text
  (`TextRenderComponent.K2_SetText` (`self.TextRender`) (`KismetTextLibrary.Conv_DoubleToText` Time "HalfToEven" false true 1 324 1 1))
  (`TextRenderComponent.K2_SetText` (`self.TextRender2`) (`KismetTextLibrary.Conv_DoubleToText` Time "HalfToEven" false true 1 324 1 1)))

(fn `UpdateLeverMaterial`
  (bind _leverhandle (`self.LeverHandle`))
  ;[1 1 1] Set lever color depending on its current state.
  (if (or (`self.IsDisabled`) (not (`self.IsInteractable`)))
    (`PrimitiveComponent.SetMaterial` _leverhandle 0 "/Game/PuzzleLogicSystem/Materials/M_LogicDeactivated.M_LogicDeactivated")
    (elif (`self.IsOnInteractCooldown`)
      (`PrimitiveComponent.SetMaterial` _leverhandle 0 "/Game/PuzzleLogicSystem/Materials/M_LogicActivated.M_LogicActivated")
      (else
        (`PrimitiveComponent.SetMaterial` _leverhandle 0 "/Game/PuzzleLogicSystem/Materials/M_DefaultMaterial.M_DefaultMaterial")))))

(fn `UserConstructionScript`
  (bind _textrender (`self.TextRender`))
  ;[1 1 1] Set starting color based on whether it's interactable or not by default.
  ; Also configures the auto-deactivate text if the lever is set to auto-deactivate.
  (`parent.UserConstructionScript`)
  (`self.UpdateLeverMaterial`)
  (if (`self.AutoDeactivate`)
    (`self.SetTimerText` (`self.AutoDeactivateTimer`))
    (`SceneComponent.SetVisibility` _textrender true true)
    (`SceneComponent.SetVisibility` (`self.TextRender2`) true true)
    (`TextRenderComponent.SetWorldSize` _textrender (`self.TimerTextSize`))
    (`TextRenderComponent.SetWorldSize` (`self.TextRender2`) (`self.TimerTextSize`))
    (`TextRenderComponent.SetTextRenderColor` (`self.TextRender`) (`self.InactiveColour`))
    (`TextRenderComponent.SetTextRenderColor` (`self.TextRender2`) (`self.InactiveColour`))
    (else
      (`SceneComponent.SetVisibility` _textrender false true)
      (`SceneComponent.SetVisibility` (`self.TextRender2`) false true))))